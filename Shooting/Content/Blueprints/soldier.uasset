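; Player-controlled soldier that moves and looks with axis inputs and plays cosmetic rifle fire while the left mouse button is held.
; Movement follows control rotation, using yaw only for forward and back.
; Pressing fire activates the muzzle flash and loop sound; releasing stops both and plays an end-shot sound, with no hit or damage logic.
; A per-tick mouse-velocity dead-zone check is unfinished and never rotates the soldier.
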(event EventTick
  (params (DeltaSeconds :type Float%20%28single-precision%29))
  (CallFunction|UpdatePlayerRotation))

(event Input|AxisEvents|InputAxisMoveForwardBack
  (params (AxisValue :type Float%20%28single-precision%29))
  (Pawn|Input|AddMovementInput (Math|Vector|GetForwardVector (Math|Rotator|MakeRotator 0.0 0.0 (.Yaw (Math|Rotator|BreakRotator (Pawn|GetControlRotation :!class /Script/Engine.Pawn))))) AxisValue false))

(event Input|AxisEvents|InputAxisMoveLeftRight
  (params (AxisValue :type Float%20%28single-precision%29))
  (Pawn|Input|AddMovementInput (Math|Vector|GetRightVector (Pawn|GetControlRotation :!class /Script/Engine.Pawn)) AxisValue false))

(event Input|AxisEvents|InputAxisLookUpDown
  (params (AxisValue :type Float%20%28single-precision%29))
  (Pawn|Input|AddControllerPitchInput AxisValue))

(event Input|AxisEvents|InputAxisLookLeftRight
  (params (AxisValue :type Float%20%28single-precision%29))
  (Pawn|Input|AddControllerYawInput AxisValue))

(event Input|MouseEvents|LeftMouseButton
  (params (Key :type Key%20Structure :default "None"))
  (:Pressed
    (bind _p_assaultrifle_mf (CallFunction|EffectsFireSoundon)))
  (:Released
    (CallFunction|EffectsFireSoundOff _p_assaultrifle_mf)))

(fn ConstructionScript)

(fn UpdatePlayerRotation
  (if (CallFunction|IsMouseDeadZone)
    _))

(fn GetMouseVelocity
  (bind _returnvalue (Game|GetPlayerController 0))
  (bind (_deltax _deltay) (Class|PlayerController|GetInputMouseDelta _returnvalue))
  (return (/ (Math|Vector2D|MakeVector2D _deltax _deltay) (Utilities|Time|GetWorldDeltaSeconds))))

(fn IsMouseDeadZone
  (return (> (Math|Vector2D|Vector2DLength (CallFunction|GetMouseVelocity)) (Variables|Default|GetMouseDeadZone))))

(fn EffectsFireSoundon
  (bind _p_assaultrifle_mf (Variables|Default|GetP_AssaultRifle_MF))
  (Components|Activation|Activate _p_assaultrifle_mf false)
  (bind _returnvalue (Audio|SpawnSound2D "/Game/Sounds/Weapon_AssaultRifle/Stereo/AssaultRifel_LoopSShoot_Cue.AssaultRifel_LoopSShoot_Cue" 1.0 1.0 0.0 0))
  (Variables|Default|SetWeaponFireSound _returnvalue)
  (return _p_assaultrifle_mf))

(fn EffectsFireSoundOff
  (params (self2 :type Actor%20Component%20Object%20Reference))
  (Components|Activation|Deactivate (Variables|Default|GetP_AssaultRifle_MF))
  (Audio|Components|Audio|Stop (Variables|Default|GetWeaponFireSound))
  (Audio|SpawnSound2D "/Game/Sounds/Weapon_AssaultRifle/Stereo/AssaultRifle_EndShoot_Cue.AssaultRifle_EndShoot_Cue" 1.0 1.0 0.0 0))